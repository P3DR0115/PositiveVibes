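; BatteryBoi is a joystick-driven player actor with a battery charge that drains as it moves.
; BeginPlay switches the numbered player's view to GameCamera, then loops to print the charge as debug text.
; Axis inputs move it along its right and forward vectors without sweep and set a shared IsMoving flag.
; Tick drains charge per frame while that flag is set and charge is non-negative; movement never checks charge.
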(event `self.ReceiveBeginPlay`
  (`PlayerController.SetViewTargetWithBlend` (`GameplayStatics.GetPlayerController` (`self.PlayerNumber`)) (`self.GameCamera`) 0.0 "VTBlend_Linear" 0.0 false)
  (`KismetSystemLibrary.Delay` 0.5 :!label _label)
  (`KismetSystemLibrary.PrintString` (`KismetStringLibrary.Conv_DoubleToString` (`self.BatteryCharge`)) true true (struct :`R` 1.0 :`B` 0.08524 :`A` 1.0) 200.0)
  (goto _label))

(event `InputAxis|JoystickX`
  (params (AxisValue :type "Float (single-precision)"))
  (if (!= AxisValue 0.0)
    (`self.K2_SetActorLocation` (+ (* (* (* (`self.GetActorRightVector`) AxisValue) (`self.MovementSpeed`)) (`GameplayStatics.GetWorldDeltaSeconds`)) (`self.K2_GetActorLocation`)))
    (set `self.isMoving` true)
    (else
      (set `self.isMoving` false :!label _label_2))))

(event `InputAxis|JoystickY`
  (params (AxisValue :type "Float (single-precision)"))
  (if (!= AxisValue 0.0)
    (`self.K2_SetActorLocation` (+ (* (* (* (`self.GetActorForwardVector`) AxisValue) (`self.MovementSpeed`)) (`GameplayStatics.GetWorldDeltaSeconds`)) (`self.K2_GetActorLocation`)))
    (set `self.isMoving` true)
    (else
      (goto _label_2))))

(event `self.ReceiveTick`
  (params (DeltaSeconds :type "Float (single-precision)"))
  (if (`self.isMoving`)
    (if (>= (`self.BatteryCharge`) 0.0)
      (set `self.BatteryCharge` (- (`self.BatteryCharge`) (`self.ChargeDeplete`))))))

(fn `AssignCamera`
  (`PlayerController.SetViewTargetWithBlend` (`GameplayStatics.GetPlayerController` (`self.PlayerNumber`)) (`self.GameCamera`) 0.0 "VTBlend_Linear" 0.0 false))

(fn `UserConstructionScript`)